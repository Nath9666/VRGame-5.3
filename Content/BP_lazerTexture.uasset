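; Laser array actor that displays nine colored cylinder beams, each aimed at its own controller mesh.
; BeginPlay pairs cylinders and controllers in matching arrays, gives each beam a dynamic gradient material tinted by Color, and scales it by WidthLazer and Distance.
; Tick re-aims every beam with a look-at rotation, offsetting pitch to align the cylinder's long axis.
; Beam length stays fixed rather than following the controller.
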(event `self.ReceiveBeginPlay`
  (bind _widthlazer (`self.WidthLazer`))
  (`|ExecutionSequence`
    (:`then_0`
      ;[1 1 1] Init Laser
      (`KismetArrayLibrary.Array_Add` (`self.AllLazer`) (`self.CylinderN5`))
      (`KismetArrayLibrary.Array_Add` (`self.AllLazer`) (`self.CylinderN1`))
      (`KismetArrayLibrary.Array_Add` (`self.AllLazer`) (`self.CylinderN9`))
      (`KismetArrayLibrary.Array_Add` (`self.AllLazer`) (`self.CylinderN8`))
      (`KismetArrayLibrary.Array_Add` (`self.AllLazer`) (`self.CylinderN7`))
      (`KismetArrayLibrary.Array_Add` (`self.AllLazer`) (`self.CylinderN6`))
      (`KismetArrayLibrary.Array_Add` (`self.AllLazer`) (`self.CylinderN4`))
      (`KismetArrayLibrary.Array_Add` (`self.AllLazer`) (`self.CylinderN3`))
      (`KismetArrayLibrary.Array_Add` (`self.AllLazer`) (`self.CylinderN2`)))
    (:`then_1`
      ;[1 1 1] Set Color
      (for _array_element (`self.AllLazer`)
        (bind _returnvalue (`PrimitiveComponent.CreateDynamicMaterialInstance` _array_element 0 "/Engine/MaterialTemplates/Gradients/Gradient_Linear.Gradient_Linear" "None"))
        (`MaterialInstanceDynamic.SetVectorParameterValue` _returnvalue "Base Color" (`self.Color`))))
    (:`then_2`
      ;[1 1 1] Init Controller
      (`KismetArrayLibrary.Array_Add` (`self.AllController`) (`self.StaticMeshN5`))
      (`KismetArrayLibrary.Array_Add` (`self.AllController`) (`self.StaticMeshN1`))
      (`KismetArrayLibrary.Array_Add` (`self.AllController`) (`self.StaticMeshN9`))
      (`KismetArrayLibrary.Array_Add` (`self.AllController`) (`self.StaticMeshN8`))
      (`KismetArrayLibrary.Array_Add` (`self.AllController`) (`self.StaticMeshN7`))
      (`KismetArrayLibrary.Array_Add` (`self.AllController`) (`self.StaticMeshN6`))
      (`KismetArrayLibrary.Array_Add` (`self.AllController`) (`self.StaticMeshN4`))
      (`KismetArrayLibrary.Array_Add` (`self.AllController`) (`self.StaticMeshN3`))
      (`KismetArrayLibrary.Array_Add` (`self.AllController`) (`self.StaticMeshN2`)))
    (:`then_3`
      (for _array_element_2 (`self.AllLazer`)
        (bind (_relativelocation_x _relativelocation_y _relativelocation_z) (`KismetMathLibrary.BreakVector` (`SceneComponent.RelativeLocation` _array_element_2)))
        (`SceneComponent.K2_SetRelativeTransform` _array_element_2 (`KismetMathLibrary.MakeTransform` (`KismetMathLibrary.MakeVector` _relativelocation_x _relativelocation_y _relativelocation_z) (struct) (`KismetMathLibrary.MakeVector` _widthlazer _widthlazer (`self.Distance`))) false false)))))

(event `self.ReceiveTick`
  (params (DeltaSeconds :type "Float (single-precision)"))
  (for (_array_element _array_index) (`self.AllLazer`)
    (bind (_returnvalue_roll _returnvalue_pitch _returnvalue_yaw) (`KismetMathLibrary.BreakRotator` (`KismetMathLibrary.FindLookAtRotation` (`SceneComponent.K2_GetComponentLocation` _array_element) (`SceneComponent.K2_GetComponentLocation` (`|GetArrayItem` (`self.AllController`) _array_index)))))
    (`SceneComponent.K2_SetWorldRotation` _array_element (`KismetMathLibrary.MakeRotator` _returnvalue_roll (+ _returnvalue_pitch 270.0) _returnvalue_yaw) false false)))

(fn `UserConstructionScript`)