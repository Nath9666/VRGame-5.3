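; Laser actor that displays nine thin, glowing beam components in a configurable color.
; The construction script fills arrays with the beams (L1–L9) and their C1–C9 counterparts.
; BeginPlay stretches each beam along Z by Distance and gives it a dynamic gradient material with LazerColor and Glow.
; Tick aims only L1 at C1, offsetting pitch to align the Z axis; the C array goes unused here.
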(event `self.ReceiveBeginPlay`
  (for _array_element (`self.Array_Lazers`)
    (`SceneComponent.K2_SetRelativeTransform` _array_element (`KismetMathLibrary.MakeTransform` (`SceneComponent.RelativeLocation` _array_element) (struct) (`KismetMathLibrary.MakeVector` 0.01 0.01 (`self.distance`))) false false)
    (bind _returnvalue (`PrimitiveComponent.CreateDynamicMaterialInstance` _array_element 0 "/Engine/MaterialTemplates/Gradients/Gradient_Linear.Gradient_Linear" "None"))
    (bind _output_get (set `self.Material` _returnvalue))
    (`MaterialInstanceDynamic.SetVectorParameterValue` _output_get "Base Color" (`KismetMathLibrary.Conv_ColorToLinearColor` (`self.LazerColor`)))
    (`MaterialInstanceDynamic.SetScalarParameterValue` _returnvalue "Glow" (`self.Glow`))))

(event `self.ReceiveTick`
  (params (DeltaSeconds :type "Float (single-precision)"))
  (bind _l1 (`self.L1`))
  (bind (_returnvalue_roll _returnvalue_pitch _returnvalue_yaw) (`KismetMathLibrary.BreakRotator` (`KismetMathLibrary.FindLookAtRotation` (`SceneComponent.K2_GetComponentLocation` _l1) (`SceneComponent.K2_GetComponentLocation` (`self.C1`)))))
  (`SceneComponent.K2_SetWorldRotation` _l1 (`KismetMathLibrary.MakeRotator` _returnvalue_roll (+ _returnvalue_pitch -90.0) _returnvalue_yaw) false false))

(fn `UserConstructionScript`
  (`|ExecutionSequence`
    (:`then_0`
      (`KismetArrayLibrary.Array_Add` (`self.Array_C_Lazers`) (`self.C1`))
      (`KismetArrayLibrary.Array_Add` (`self.Array_C_Lazers`) (`self.C2`))
      (`KismetArrayLibrary.Array_Add` (`self.Array_C_Lazers`) (`self.C3`))
      (`KismetArrayLibrary.Array_Add` (`self.Array_C_Lazers`) (`self.C4`))
      (`KismetArrayLibrary.Array_Add` (`self.Array_C_Lazers`) (`self.C5`))
      (`KismetArrayLibrary.Array_Add` (`self.Array_C_Lazers`) (`self.C6`))
      (`KismetArrayLibrary.Array_Add` (`self.Array_C_Lazers`) (`self.C7`))
      (`KismetArrayLibrary.Array_Add` (`self.Array_C_Lazers`) (`self.C8`))
      (`KismetArrayLibrary.Array_Add` (`self.Array_C_Lazers`) (`self.C9`)))
    (:`then_1`
      (`KismetArrayLibrary.Array_Add` (`self.Array_Lazers`) (`self.L1`))
      (`KismetArrayLibrary.Array_Add` (`self.Array_Lazers`) (`self.L2`))
      (`KismetArrayLibrary.Array_Add` (`self.Array_Lazers`) (`self.L3`))
      (`KismetArrayLibrary.Array_Add` (`self.Array_Lazers`) (`self.L4`))
      (`KismetArrayLibrary.Array_Add` (`self.Array_Lazers`) (`self.L5`))
      (`KismetArrayLibrary.Array_Add` (`self.Array_Lazers`) (`self.L6`))
      (`KismetArrayLibrary.Array_Add` (`self.Array_Lazers`) (`self.L7`))
      (`KismetArrayLibrary.Array_Add` (`self.Array_Lazers`) (`self.L8`))
      (`KismetArrayLibrary.Array_Add` (`self.Array_Lazers`) (`self.L9`)))))