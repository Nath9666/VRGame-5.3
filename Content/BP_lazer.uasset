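; Laser actor that fires nine colored beam effects outward from its location.
; BeginPlay gathers the effect and controller mesh components into paired arrays, applies a color, then sets each beam's End from the matching mesh's relative location scaled by Distance.
; Each beam also runs a multi line trace whose result is unused.
; Endpoints are set once, as Tick is empty and a look-at rotation snippet is disconnected.
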(event `self.ReceiveBeginPlay`
  (bind _returnvalue (`self.K2_GetActorLocation`))
  (bind _alllazer (`self.AllLazer`))
  (`|ExecutionSequence`
    (:`then_0`
      (`KismetArrayLibrary.Array_Add` (`self.AllLazer`) (`self.LazerN5`))
      (`KismetArrayLibrary.Array_Add` _alllazer (`self.LazerN1`))
      (`KismetArrayLibrary.Array_Add` _alllazer (`self.LazerN9`))
      (`KismetArrayLibrary.Array_Add` (`self.AllLazer`) (`self.LazerN8`))
      (`KismetArrayLibrary.Array_Add` (`self.AllLazer`) (`self.LazerN7`))
      (`KismetArrayLibrary.Array_Add` (`self.AllLazer`) (`self.LazerN6`))
      (`KismetArrayLibrary.Array_Add` (`self.AllLazer`) (`self.LazerN4`))
      (`KismetArrayLibrary.Array_Add` (`self.AllLazer`) (`self.LazerN3`))
      (`KismetArrayLibrary.Array_Add` (`self.AllLazer`) (`self.LazerN2`)))
    (:`then_1`
      (for _array_element (`self.AllLazer`)
        (`FXSystemComponent.SetColorParameter` _array_element "Color" (`self.Param`))))
    (:`then_2`
      (`KismetArrayLibrary.Array_Add` (`self.AllController`) (`self.StaticMeshN5`))
      (`KismetArrayLibrary.Array_Add` (`self.AllController`) (`self.StaticMeshN1`))
      (`KismetArrayLibrary.Array_Add` (`self.AllController`) (`self.StaticMeshN9`))
      (`KismetArrayLibrary.Array_Add` (`self.AllController`) (`self.StaticMeshN8`))
      (`KismetArrayLibrary.Array_Add` (`self.AllController`) (`self.StaticMeshN7`))
      (`KismetArrayLibrary.Array_Add` (`self.AllController`) (`self.StaticMeshN6`))
      (`KismetArrayLibrary.Array_Add` (`self.AllController`) (`self.StaticMeshN4`))
      (`KismetArrayLibrary.Array_Add` (`self.AllController`) (`self.StaticMeshN3`))
      (`KismetArrayLibrary.Array_Add` (`self.AllController`) (`self.StaticMeshN2`)))
    (:`then_3`
      (for (_array_element_2 _array_index) (`self.AllLazer`)
        (bind _returnvalue_2 (+ _returnvalue (* (`SceneComponent.RelativeLocation` (`|GetArrayItem` (`self.AllController`) _array_index)) (`self.Distance`))))
        (`KismetSystemLibrary.LineTraceMulti` _returnvalue _returnvalue_2 "TraceTypeQuery1" true)
        (`FXSystemComponent.SetVectorParameter` _array_element_2 "End" _returnvalue_2)))))

(event `self.ReceiveTick`
  (params (DeltaSeconds :type "Float (single-precision)")))

(fn `UserConstructionScript`)