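; BP_FulguroBeam is a rotating light-show fixture with left (G) and right (D) groups of four spotlights and four fog cones, plus two lasers.
; BeginPlay applies color and power to the lights, sets dynamic fog-cone materials, and spawns a Bp_Lazetr at each side joint.
; Tick yaws the central joint at half Speed and both side joints at full Speed, then copies joint transforms onto the unattached lasers.
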(event `self.ReceiveBeginPlay`
  (`|ExecutionSequence`
    (:`then_0`
      ;[1 1 1] Init Light and Color
      (`self.GetAllGLight`)
      (`self.GetAllDLight`)
      (bind _alllight (`self.GetAllLight`))
      (for _array_element _alllight
        (`LightComponent.SetLightColor` _array_element (`self.LightColor`) true)
        (`LightComponent.SetIntensity` _array_element (`self.Power`))))
    (:`then_1`
      ;[1 1 1] Init Fog and color
      (`self.GetAllDFog`)
      (`self.GetAllGFog`)
      (`self.GetAllFog`)
      (for _array_element_2 (`self.AllFog`)
        (bind _returnvalue (`PrimitiveComponent.CreateDynamicMaterialInstance` _array_element_2 0 "/Game/FulguroBeam/material/MI_Transparent_Inst.MI_Transparent_Inst" "None"))
        (`MaterialInstanceDynamic.SetVectorParameterValue` _returnvalue "Base Color" (`self.LightColor`))
        (`MaterialInstanceDynamic.SetScalarParameterValue` _returnvalue "Distance" (`self.Fumee`))))
    (:`then_2`
      (bind _returnvalue_2 (`|SpawnActorFromClass` "/Game/Bp_Lazetr.Bp_Lazetr_C" (`SceneComponent.K2_GetComponentToWorld` (`self.Join_G`)) "AlwaysSpawn" "MultiplyWithRoot" null (`self.LazerDistance`) (`KismetMathLibrary.Conv_LinearColorToColor` (`self.LazerColor`)) 1.0 null))
      (set `self.Lazer_G` _returnvalue_2)
      (bind _returnvalue_3 (`|SpawnActorFromClass` "/Game/Bp_Lazetr.Bp_Lazetr_C" (`SceneComponent.K2_GetComponentToWorld` (`self.Joint_D`)) "AlwaysSpawn" "MultiplyWithRoot" null (`self.LazerDistance`) (`KismetMathLibrary.Conv_LinearColorToColor` (`self.LazerColor`)) 1.0 null))
      (set `self.Lazer_D` _returnvalue_3))))

(event `self.ReceiveTick`
  (params (DeltaSeconds :type "Float (single-precision)"))
  (bind _join_g (`self.Join_G`))
  (bind _joint_d (`self.Joint_D`))
  (`|ExecutionSequence`
    (:`then_0`
      (`self.RotateProjector` (`self.Jointure`) (/ (`self.Speed`) 2.0) (`GameplayStatics.GetWorldDeltaSeconds`)))
    (:`then_1`
      (`self.RotateProjector` (`self.Join_G`) (`self.Speed`) (`GameplayStatics.GetWorldDeltaSeconds`))
      (`self.RotateProjector` (`self.Joint_D`) (`self.Speed`) (`GameplayStatics.GetWorldDeltaSeconds`)))
    (:`then_2`
      (`SceneComponent.K2_SetWorldLocationAndRotation` (`Actor.RootComponent` (`self.Lazer_G`)) (`SceneComponent.K2_GetComponentLocation` _join_g) (`SceneComponent.K2_GetComponentRotation` _join_g) false false)
      (`SceneComponent.K2_SetWorldLocationAndRotation` (`Actor.RootComponent` (`self.Lazer_D`)) (`SceneComponent.K2_GetComponentLocation` _joint_d) (`SceneComponent.K2_GetComponentRotation` _joint_d) false false))))

(fn `GetAllDFog`
  (`|ExecutionSequence`
    (:`then_0`
      (`KismetArrayLibrary.Array_Add` (`self.AllFog_D`) (`self.Cone4`)))
    (:`then_1`
      (`KismetArrayLibrary.Array_Add` (`self.AllFog_D`) (`self.Cone5`)))
    (:`then_2`
      (`KismetArrayLibrary.Array_Add` (`self.AllFog_D`) (`self.Cone6`)))
    (:`then_3`
      (`KismetArrayLibrary.Array_Add` (`self.AllFog_D`) (`self.Cone7`)))))

(fn `GetAllDLight`
  (`|ExecutionSequence`
    (:`then_0`
      (`KismetArrayLibrary.Array_Add` (`self.Projectors_D`) (`self.SpotLight2`)))
    (:`then_1`
      (`KismetArrayLibrary.Array_Add` (`self.Projectors_D`) (`self.SpotLight3`)))
    (:`then_2`
      (`KismetArrayLibrary.Array_Add` (`self.Projectors_D`) (`self.SpotLight1`)))
    (:`then_3`
      (`KismetArrayLibrary.Array_Add` (`self.Projectors_D`) (`self.SpotLight`)))))

(fn `GetAllFog`
  (bind _allfog (`self.AllFog`))
  (`|ExecutionSequence`
    (:`then_0`
      (for _array_element (`self.AllFog_D`)
        (`KismetArrayLibrary.Array_Add` _allfog _array_element)))
    (:`then_1`
      (for _array_element_2 (`self.AllFog_G`)
        (`KismetArrayLibrary.Array_Add` _allfog _array_element_2)))))

(fn `GetAllGFog`
  (bind _allfog_g (`self.AllFog_G`))
  (`|ExecutionSequence`
    (:`then_0`
      (`KismetArrayLibrary.Array_Add` _allfog_g (`self.Cone3`)))
    (:`then_1`
      (`KismetArrayLibrary.Array_Add` _allfog_g (`self.Cone2`)))
    (:`then_2`
      (`KismetArrayLibrary.Array_Add` _allfog_g (`self.Cone1`)))
    (:`then_3`
      (`KismetArrayLibrary.Array_Add` _allfog_g (`self.Cone`)))))

(fn `GetAllGLight`
  (`|ExecutionSequence`
    (:`then_0`
      (`KismetArrayLibrary.Array_Add` (`self.Projectors_G`) (`self.SpotLight4`)))
    (:`then_1`
      (`KismetArrayLibrary.Array_Add` (`self.Projectors_G`) (`self.SpotLight5`)))
    (:`then_2`
      (`KismetArrayLibrary.Array_Add` (`self.Projectors_G`) (`self.SpotLight6`)))
    (:`then_3`
      (`KismetArrayLibrary.Array_Add` (`self.Projectors_G`) (`self.SpotLight7`)))))

(fn `GetAllLight`
  (returns (AllLight :type "Array of SpotLightComponent Object Reference"))
  (bind _alllight (`self.AllLight`))
  (`|ExecutionSequence`
    (:`then_0`
      (for _array_element (`self.Projectors_G`)
        (`KismetArrayLibrary.Array_Add` _alllight _array_element)))
    (:`then_1`
      (for _array_element_2 (`self.Projectors_D`)
        (`KismetArrayLibrary.Array_Add` _alllight _array_element_2)))
    (:`then_2`
      (return (`self.AllLight`)))))

(fn `RotateProjector`
  (params (Projector_Name :type "StaticMeshComponent Object Reference") (Speed :type "Float (double-precision)") (DeltaTime :type "Float (double-precision)"))
  (`SceneComponent.K2_AddLocalRotation` Projector_Name (`KismetMathLibrary.MakeRotator` 0.0 0.0 (* Speed DeltaTime)) false false))

(fn `UserConstructionScript`)